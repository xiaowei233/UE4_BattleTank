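; Player tank Blueprint that sets up its barrel and handles orbit camera aiming input.
; On BeginPlay it assigns the barrel mesh to the TankBarrel component and passes that component to SetBarrelReference.
; The AimAzimuth axis yaws the Scene component and AimElevation pitches the SpringArm, splitting camera rotation across two components.
; Both rotations scale raw axis values by fixed sensitivities, without delta time.
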(event `self.ReceiveBeginPlay`
  (bind _tankbarrel (`self.TankBarrel`))
  (`StaticMeshComponent.SetStaticMesh` _tankbarrel "/Game/Mesh/tank_fbx_Barrel.tank_fbx_Barrel")
  (`self.SetBarrelReference` _tankbarrel))

(event `InputAxis|AimAzimuth`
  (params (AxisValue :type "Float (single-precision)"))
  ;[1 1 1] Camera Input Biding
  (`SceneComponent.K2_AddLocalRotation` (`self.Scene`) (`KismetMathLibrary.MakeRotator` 0.0 0.0 (* AxisValue 0.8)) false false))

(event `InputAxis|AimElevation`
  (params (AxisValue :type "Float (single-precision)"))
  ;[1 1 1] Camera Input Biding
  (`SceneComponent.K2_AddLocalRotation` (`self.SpringArm`) (`KismetMathLibrary.MakeRotator` 0.0 (* AxisValue 0.6)) false false))

(fn `UserConstructionScript`)