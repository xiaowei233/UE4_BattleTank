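; DayNight Blueprint that runs a continuous day-night cycle by rotating the directional light and skylight and updating the sky sphere's sun direction.
; Each Tick turns both lights by a fixed step, not scaled by delta time, so cycle speed follows frame rate.
; The sun's pitch selects Day or Night, which ease both light intensities toward bright or dim targets with FInterpTo.
; Sky sphere recoloring in Night is disconnected and never runs.
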(event `self.ReceiveTick`
  (params (DeltaSeconds :type "Float (single-precision)"))
  (bind _returnvalue (`GameplayStatics.GetWorldDeltaSeconds`))
  (bind (_returnvalue_roll _returnvalue_pitch) (`KismetMathLibrary.BreakRotator` (`self.K2_GetActorRotation` (`self.DirectionalLight`))))
  (`self.K2_AddActorLocalRotation` (`self.DirectionalLight`) (struct :`Pitch` 0.2) false false)
  (`/Engine/EngineSky/BP_Sky_Sphere.UpdateSunDirection` (`self.SkySphere`))
  (`self.K2_AddActorLocalRotation` (`self.SkyLight`) (struct :`Pitch` 0.2) false false)
  (if (> _returnvalue_pitch 0.0)
    (`self.Night` _returnvalue)
    (else
      (`self.Day` _returnvalue))))

(fn `Day`
  (params (DeltaTime :type "Float (double-precision)"))
  (bind _lightcomponent (`Light.LightComponent` (`self.DirectionalLight`)))
  (bind _lightcomponent_2 (`SkyLight.LightComponent` (`self.SkyLight`)))
  (`LightComponent.SetIntensity` _lightcomponent (`KismetMathLibrary.FInterpTo` (`LightComponentBase.Intensity` _lightcomponent) 3.141593 DeltaTime 1.0))
  (`SkyLightComponent.SetIntensity` _lightcomponent_2 (`KismetMathLibrary.FInterpTo` (`LightComponentBase.Intensity` _lightcomponent_2) 1.0 DeltaTime 1.0)))

(fn `Night`
  (params (DeltaTime :type "Float (double-precision)"))
  (bind _lightcomponent (`Light.LightComponent` (`self.DirectionalLight`)))
  (bind _lightcomponent_2 (`SkyLight.LightComponent` (`self.SkyLight`)))
  (`LightComponent.SetIntensity` _lightcomponent (`KismetMathLibrary.FInterpTo` (`LightComponentBase.Intensity` _lightcomponent) 0.01 DeltaTime 1.0))
  (`SkyLightComponent.SetIntensity` _lightcomponent_2 (`KismetMathLibrary.FInterpTo` (`LightComponentBase.Intensity` _lightcomponent_2) 0.1 DeltaTime 1.0)))

(fn `UserConstructionScript`)